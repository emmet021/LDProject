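; Placeable trigger switch that, when remotely interacted with, can drive a list of linked actors and a referenced door.
; RemoteInteract flip-flops the Active flag and calls the door's Wallswitch the first time it turns on.
; RemoteInteractResponse plays a deactivate sound when inactive; when active, it plays an activate sound and messages each linked actor with an elevator direction through a delayed loop, with another once-only Wallswitch call.
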(event `self.RemoteInteractResponse`
  (if (`self.active`)
    (`GameplayStatics.PlaySoundAtLocation` (`self.ActivateSound`) (`self.K2_GetActorLocation`) (struct) 3.0 1.0 0.0 null null null null)
    (bind _array_element (`/Game/Blueprints/MAcros/StandardMacros.ForEachLoop_WithDelay` (`self.SwitchActors`) (`self.Delay Amount`))
      (:`LoopBody`
        (message `/Game/Blueprints/Placeables/interactions/Interact_BI.Remote Interact` _array_element (`self.ElevatorDirection`))
        (`/Engine/EditorBlueprintResources/StandardMacros.DoOnce` false
          (:`Completed`
            (`/Game/Levels/MovingDoor.Wallswitch` (`self.door refernace`))))))
    (else
      (`GameplayStatics.PlaySoundAtLocation` (`self.Deactivate Sound`) (`self.K2_GetActorLocation`) (struct) 3.0 1.0 0.5 null null null null))))

(event `/Game/Blueprints/Placeables/interactions/Interact_BI.Remote Interact`
  (params (Direction :type "EDirection Enum" :default "Left"))
  (`/Engine/EditorBlueprintResources/StandardMacros.FlipFlop`
    (:`A`
      (set `self.active` true)
      (`/Engine/EditorBlueprintResources/StandardMacros.DoOnce` false
        (:`Completed`
          (`/Game/Levels/MovingDoor.Wallswitch` (`self.door refernace`)))))
    (:`B`
      (set `self.active` false))))

(fn `UserConstructionScript`
  (`parent.UserConstructionScript`))